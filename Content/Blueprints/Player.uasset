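; Player character for a twin-stick shooter that moves, aims, fires and respawns on death.
; On BeginPlay it adds the HUD, attaches a spawned weapon to GunSocket and gives TwinStickMode its spawn transform.
; Look input past a deadzone rotates the controller and fires, slowing movement; the Shooting flag is inverted, true while not firing.
; Lethal damage flags a cutscene, disables input, then after a delay requests respawn and destroys weapon and pawn.
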(event `/Game/Blueprints/damageInterface.Affect Health`
  (params (Delta :type "Float (single-precision)"))
  (`self.CalculateHealth` Delta)
  (if (`self.isDead`)
    (set `self.startCutscene` true)
    (`self.DisableInput` null)
    (`KismetSystemLibrary.Delay` 4.0)
    (`/Game/Blueprints/TwinStickMode.Respawn Player` (`self.GameMode`))
    (`self.K2_DestroyActor` (`self.Weapon`))
    (`self.K2_DestroyActor` self)))

(event `InputAxis|MoveUp`
  (params (AxisValue :type "Float (single-precision)"))
  ;[1 1 1] Movement Code
  (if (`self.Shooting`)
    (`self.AddMovementInput` (1.0 0.0 0.0) AxisValue)
    (else
      (`self.AddMovementInput` (0.6 0.0 0.0) AxisValue))))

(event `InputAxis|LookUp`
  (params (AxisValue :type "Float (single-precision)"))
  (bind _weapon (`self.Weapon`))
  ;[1 1 1] Rotation Code
  (bind _returnvalue (`KismetMathLibrary.MakeVector` AxisValue (stale `InputAxis|LookRight` AxisValue)))
  (if (> (`KismetMathLibrary.VSize` _returnvalue) 0.25) :!label _label
    (`Controller.SetControlRotation` (`self.GetController`) (`KismetMathLibrary.Conv_VectorToRotator` _returnvalue))
    (`/Game/Blueprints/PlayerWeapon.BeginShooting` _weapon)
    (set `self.Shooting` false)
    (else
      (`/Game/Blueprints/PlayerWeapon.StopShooting` _weapon)
      (set `self.Shooting` true))))

(event `InputAxis|MoveRight`
  (params (AxisValue :type "Float (single-precision)"))
  ;[1 1 1] Movement Code
  (if (`self.Shooting`)
    (`self.AddMovementInput` (0.0 1.0 0.0) AxisValue)
    (else
      (`self.AddMovementInput` (0.0 0.6 0.0) AxisValue))))

(event `InputAxis|LookRight`
  (params (AxisValue :type "Float (single-precision)"))
  ;[1 1 1] Rotation Code
  (goto _label))

(event `self.ReceiveBeginPlay`
  (bind _mesh (`self.Mesh`))
  (bind _returnvalue (`|CreateWidget` "/Game/HUD/PlayerHUD.PlayerHUD_C"))
  (`UserWidget.AddToViewport` _returnvalue 0)
  (`|ExecutionSequence`
    (:`then_0`
      (bind _returnvalue_2 (`|SpawnActorFromClass` "/Game/Blueprints/PlayerWeapon.PlayerWeapon_C" (`SceneComponent.K2_GetComponentToWorld` _mesh) "Undefined" "OverrideRootScale"))
      (bind _output_get (set `self.Weapon` _returnvalue_2))
      (`self.K2_AttachRootComponentTo` (`self.Weapon`) _mesh "GunSocket" "SnapToTarget" true)
      (`self.K2_AttachRootComponentTo` _output_get _mesh "GunSocket" "SnapToTarget" true))
    (:`then_1`
      (bind _astwin_stick_mode (cast `/Game/Blueprints/TwinStickMode` (`GameplayStatics.GetGameMode`)))
      (bind _output_get_2 (set `self.GameMode` _astwin_stick_mode))
      (set `/Game/Blueprints/TwinStickMode.Player Spawn Transform` (`self.GetTransform`) _output_get_2))))

(event `self.ReceiveActorBeginOverlap`
  (params (OtherActor :type "Actor Object Reference")))

(fn `UserConstructionScript`)