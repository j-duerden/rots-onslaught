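; PlayerWeapon is an automatic weapon Blueprint that fires bullets for as long as shooting is active.
; BeginShooting passes through a DoOnce gate, fires immediately, then starts a looping timer on Fire at an interval derived from RoundsPerSec.
; Each Fire spawns a Bullet at the BulletSpawnpoint transform and plays a 2D gunshot sound.
; StopShooting clears the timer and resets the gate.
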(event `BeginShooting`
  ;[1 1 1] Firing Code
  (`/Engine/EditorBlueprintResources/StandardMacros.DoOnce` false :!label _label
    (:`Completed`
      (`self.Fire`)
      (bind _returnvalue (`KismetSystemLibrary.K2_SetTimer` null "Fire" (/ 1.0 (`self.RoundsPerSec`)) true))
      (set `self.Firing Timer` _returnvalue))))

(event `StopShooting`
  ;[1 1 1] Firing Code
  (`KismetSystemLibrary.K2_ClearTimerHandle` (`self.Firing Timer`))
  (goto _label :!via `Reset`))

(event `Fire`
  ;[1 1 1] Firing Code
  (`|SpawnActorFromClass` "/Game/Blueprints/Bullet.Bullet_C" (`SceneComponent.K2_GetComponentToWorld` (`self.Bullet_Spawnpoint`)) "Undefined" "OverrideRootScale")
  (`GameplayStatics.PlaySound2D` "/Game/Sounds/GunshotCue.GunshotCue"))

(event `self.ReceiveBeginPlay`)

(event `self.ReceiveActorBeginOverlap`
  (params (OtherActor :type "Actor Object Reference")))

(event `self.ReceiveTick`
  (params (DeltaSeconds :type "Float (single-precision)")))

(fn `UserConstructionScript`)