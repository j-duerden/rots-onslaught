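; Bullet is a projectile Blueprint that deals damage to what it overlaps and plays a 2D sound when it spawns.
; On overlap, it sends its Damage through the DamageInterface's AffectHealthMessage to implementers not tagged Friendly, then destroys itself.
; Overlapping an actor without the interface also destroys the bullet, while Friendly implementers leave it intact and take no damage.
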(event `self.ReceiveBeginPlay`
  (`/Engine/EditorBlueprintResources/StandardMacros.DoOnce` false
    (:`Completed`
      (`GameplayStatics.PlaySound2D` null))))

(event `self.ReceiveActorBeginOverlap`
  (params (OtherActor :type "Actor Object Reference"))
  (if (`KismetSystemLibrary.DoesImplementInterface` OtherActor "/Game/Blueprints/damageInterface.damageInterface_C")
    (if (not (`self.ActorHasTag` OtherActor "Friendly"))
      (message `/Game/Blueprints/damageInterface.Affect Health` OtherActor (`self.Damage`))
      (`self.K2_DestroyActor` :!label _label))
    (else
      (goto _label))))

(event `self.ReceiveBeginPlay`)

(event `self.ReceiveTick`
  (params (DeltaSeconds :type "Float (single-precision)")))

(fn `UserConstructionScript`)