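; Melee enemy for a twin-stick game that hurts the player on contact and awards a point when killed.
; Overlapping the player starts a looping timer that deals damage at the attacks-per-second rate until the overlap ends.
; Health changes run through CalculateHealth; death increments TwinStickMode points and destroys the actor, spawning smoke on destruction.
; The construction script lowers walk speed relative to its current value.
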(event `self.ReceiveDestroyed`
  (`GameplayStatics.SpawnEmitterAtLocation` "/Game/Particles/DeathSmoke.DeathSmoke" (`self.K2_GetActorLocation`)))

(event `/Game/Blueprints/damageInterface.Affect Health`
  (params (Delta :type "Float (single-precision)"))
  ;[1 1 1] Enemy Health Code
  (`self.CalculateHealth` Delta)
  (if (`self.isDead`)
    (bind _astwin_stick_mode (cast `/Game/Blueprints/TwinStickMode` (`GameplayStatics.GetGameMode`)))
    (set `/Game/Blueprints/TwinStickMode.Points` (+ (`/Game/Blueprints/TwinStickMode.Points` _astwin_stick_mode) 1) _astwin_stick_mode)
    (`self.K2_DestroyActor`)))

(event `self.ReceiveActorBeginOverlap`
  (params (OtherActor :type "Actor Object Reference"))
  ;[1 1 1] Enemy Attack Code
  (bind _asplayer (cast `/Game/Blueprints/Player` OtherActor))
  (set `self.PlayerCharacter` _asplayer)
  (bind _returnvalue (`KismetSystemLibrary.K2_SetTimer` null "DamagePlayer" (/ 1.0 (`self.Attacks Per Sec`)) true))
  (set `self.Hit` _returnvalue))

(event `DamagePlayer`
  ;[1 1 1] Enemy Attack Code
  (`/Game/Blueprints/Player.Affect Health` (`self.PlayerCharacter`) (`self.Damage`)))

(event `self.ReceiveActorEndOverlap`
  (params (OtherActor :type "Actor Object Reference"))
  ;[1 1 1] Enemy Attack Code
  (if (== OtherActor (`self.PlayerCharacter`))
    (`KismetSystemLibrary.K2_ClearTimerHandle` (`self.Hit`))))

(event `self.ReceiveBeginPlay`)

(event `self.ReceiveTick`
  (params (DeltaSeconds :type "Float (single-precision)")))

(fn `UserConstructionScript`
  (set `CharacterMovementComponent.MaxWalkSpeed` (- (`CharacterMovementComponent.MaxWalkSpeed` (`self.CharacterMovement`)) 75.0) (`self.CharacterMovement`)))